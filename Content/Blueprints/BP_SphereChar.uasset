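; BP_SphereChar is a sphere character Blueprint with an unfinished rolling-movement prototype; none of its event graph logic runs.
; The disconnected nodes derive a forward vector from control yaw for movement input and rotate CharMesh, scaling the spin by the inverse of capsule radius.
; Both calculations multiply by a zero vector, a debug print is also unwired, and the construction script is empty.
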(fn ConstructionScript)